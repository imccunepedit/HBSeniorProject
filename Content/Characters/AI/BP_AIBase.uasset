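; Base AI character that talks to the player and ties its text to the player's score, with name label and tag set at construction.
; It listens for the player's score updates, advancing a name-plus-number text key and progress index at listed scores.
; Ending an interaction at the expected score updates that score once per stage.
; Tick rotates the label via LookAtCamera, whose look-at calculation is left unconnected.
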(event `self.ReceiveBeginPlay`
  (`|ExecutionSequence`
    (:`then_2`
      ;[1 1 1] set initial text index based on name
      (set `self.TextIndex` (`KismetStringLibrary.Conv_StringToName` (`KismetStringLibrary.Concat_StrStr` (`self.Name`) (`KismetStringLibrary.Conv_IntToString` (`self.TextIndexNum`))))))
    (:`then_3`
      ;[1 1 1] Listen for dispatch event
      (bind _asbp_player_character (cast `/Game/Characters/Player/BP_PlayerCharacter` (`GameplayStatics.GetPlayerCharacter` 0)))
      (bind _output_get (set `self.BP_PlayerCharacterRef` _asbp_player_character))
      (add `/Game/Characters/Player/BP_PlayerCharacter.ScoreUpdate` _output_get (delegate `ScoreUpdate`)))))

(event `self.ReceiveTick`
  (params (DeltaSeconds :type "Float (single-precision)"))
  ;[1 1 1] Show the text and aim at camera
  (`|ExecutionSequence`
    (:`then_1`
      (`SceneComponent.K2_SetWorldRotation` (`self.NameText`) (`KismetMathLibrary.FindLookAtRotation` (`SceneComponent.K2_GetComponentLocation` (`self.NameText`)) (`SceneComponent.K2_GetComponentLocation` (`Character.CapsuleComponent` (`GameplayStatics.GetPlayerCharacter` 0)))) false false))))

(event `ScoreUpdate`
  (params (Score :type Integer))
  ;[1 1 1] cycle text and change what the score to progress when talking is based
  (`|ExecutionSequence`
    (:`then_0`
      (if (`KismetArrayLibrary.Array_Contains` (`self.ScoresToChangeText`) Score)
        (`self.CycleText`)
        (`/Engine/EditorBlueprintResources/StandardMacros.IncrementInt` (`self.ScoresToProgressIndex`)
          (:`  `
            (set `self.HasTalked` false)))))))

(event `EndInteract`
  ;[1 1 1] check wether ai has interacted with player to update score if relevent
  (if (and (not (`self.HasTalked`)) (== (`/Game/Characters/Player/BP_PlayerCharacter.Score` (`self.BP_PlayerCharacterRef`)) (`|GetArrayItem` (`self.ScoresToProgress`) (`self.ScoresToProgressIndex`))))
    (`/Game/Characters/Player/BP_PlayerCharacter.UpdateScore` (`self.BP_PlayerCharacterRef`))
    (set `self.HasTalked` true)))

(event `CycleText`
  ;[1 1 1] Change the index for the characters text
  (bind _result (`/Engine/EditorBlueprintResources/StandardMacros.IncrementInt` (`self.TextIndexNum`))
    (:`  `
      (set `self.TextIndex` (`KismetStringLibrary.Conv_StringToName` (`KismetStringLibrary.Concat_StrStr` (`self.Name`) (`KismetStringLibrary.Conv_IntToString` _result)))))))

(fn `UserConstructionScript`
  (bind _tags (`self.Tags`))
  (bind _name (`self.Name`))
  (bind _returnvalue (`KismetStringLibrary.Conv_StringToName` _name))
  (`|ExecutionSequence`
    (:`then_0`
      (`TextRenderComponent.K2_SetText` (`self.NameText`) (`KismetTextLibrary.Conv_StringToText` (`self.Name`)))
      (if (not (`KismetArrayLibrary.Array_Contains` _tags _returnvalue))
        (`KismetArrayLibrary.Array_Add` _tags _returnvalue)
        (if (`KismetStringLibrary.NotEqual_StrStr` _name "Base")
          (`KismetArrayLibrary.Array_RemoveItem` _tags (`KismetStringLibrary.Conv_StringToName` "Base")))))))